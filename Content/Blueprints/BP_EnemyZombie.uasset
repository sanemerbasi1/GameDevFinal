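; BP_EnemyZombie is an enemy zombie Blueprint that pursues the player and has a health bar widget.
; On BeginPlay, if the widget object is valid, it passes itself to WBP_EnemyHealth and starts a looping one-second timer.
; The timer calls FollowPlayer on the player's BP_Avatar, avoiding Tick.
; OnHealthChanged forwards the new health through CallOnHealthChangedDispatch.
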(event `self.OnHealthChanged`
  (params (NewHealth :type "Float (single-precision)"))
  (`self.OnHealthChangedDispatch` NewHealth))

(event `self.ReceiveBeginPlay`
  (bind _returnvalue (`WidgetComponent.GetUserWidgetObject` (`self.HealthBarWidget`)))
  (`/Engine/EditorBlueprintResources/StandardMacros.IsValid` _returnvalue
    (:`Is Valid`
      (set `/Game/Blueprints/Widgets/WBP_EnemyHealth.BP_EnemyZombie` self (cast `/Game/Blueprints/Widgets/WBP_EnemyHealth` _returnvalue :!pure true))
      (`KismetSystemLibrary.K2_SetTimerDelegate` (delegate `CustomEvent`) 1.0 true))))

(event `CustomEvent`
  (`self.FollowPlayer` (cast `/Game/Blueprints/BP_Avatar` (`GameplayStatics.GetPlayerCharacter` 0) :!pure true)))

(fn `UserConstructionScript`)