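; BP_NetGameMode is a game mode that spawns zombie enemies and triggers victory when all have died.
; On BeginPlay it spawns a BP_EnemyZombie at each "EnemySpawn" tagged spawner, stores it in an array and binds its Died event.
; Each death removes the last array entry, so the array serves as a counter.
; At zero, the local avatar's victory UI replaces its game UI and the mouse cursor appears.
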(event `VictoryWidget`)

(event `Died_Event`)

(event `Spawner`
  (bind _returnvalue (`self.GetSpawnersByTag` "EnemySpawn"))
  (for _array_element _returnvalue
    (bind (_returnvalue_location _returnvalue_rotation) (`KismetMathLibrary.BreakTransform` (`self.GetTransform` _array_element)))
    (bind _returnvalue_2 (`self.SpawnEnemy` "/Game/Blueprints/BP_EnemyZombie.BP_EnemyZombie_C" _returnvalue_location _returnvalue_rotation))
    (bind _returnvalue_3 (`KismetArrayLibrary.Array_Add` (`self.BP_Zombie`) _returnvalue_2))
    (`KismetSystemLibrary.PrintString` (`KismetStringLibrary.Conv_IntToString` _returnvalue_3))
    (add `/Game/Blueprints/BP_EnemyZombie.Died` (cast `/Game/Blueprints/BP_EnemyZombie` _returnvalue_2 :!pure true) (delegate `Died_Event_0`))))

(event `Died_Event_0`
  (bind _asbp_avatar (cast `/Game/Blueprints/BP_Avatar` (`GameplayStatics.GetPlayerCharacter` 0) :!pure true))
  (`KismetArrayLibrary.Array_Remove` (`self.BP_Zombie`) (- (`KismetArrayLibrary.Array_Length` (`self.BP_Zombie`)) 1))
  (if (== 0 (`KismetArrayLibrary.Array_Length` (`self.BP_Zombie`)))
    (`UserWidget.AddToViewport` (`/Game/Blueprints/BP_Avatar.VictoryUI` _asbp_avatar) 0)
    (`Widget.RemoveFromParent` (`/Game/Blueprints/BP_Avatar.GameUI` _asbp_avatar))
    (set `PlayerController.bShowMouseCursor` true (`GameplayStatics.GetPlayerController` 0))))

(event `self.ReceiveBeginPlay`
  (`self.Spawner`))

(fn `UserConstructionScript`)